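; Actor component that inflates its owner like a balloon, morphing a mesh and lifting it with physics.
; AddInflate raises a capped target that Tick climbs toward, calling CallHitMax at maximum, then clearing the target so it deflates.
; Inflation drives the "Inflate" morph target and a runtime-spawned thruster held at fixed world rotation.
; Thrust scales with mesh mass and inflation relative to ZeroWeightLimit.
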(event EventBeginPlay
  (bind _returnvalue (Game|AddComponentbyClass (Components|GetOwner) "/Script/Engine.PhysicsThrusterComponent" false))
  (Variables|Default|SetThruster _returnvalue))

(event EventTick
  (params (DeltaSeconds :type Float%20%28single-precision%29))
  (bind _thruster (Variables|Default|GetThruster))
  (CallFunction|UpdateCurrentInflation DeltaSeconds)
  (Utilities|IsValid _thruster
    (:Is%20Valid
      (Transformation|SetWorldRotation _thruster "-90.000000,0.000000,0.000000" false false)
      (CallFunction|UpdateMorph)
      (CallFunction|UpdatePhysics))))

(fn AddInflate
  (params (Inflate_amount :type Float%20%28double-precision%29))
  (Utilities|FlowControl|Sequence
    (:then_0
      (if (> (Variables|Default|GetCurrent_Inflate) (Variables|Default|GetTarget_Inflate))
        (Variables|Default|SetTarget_Inflate (Variables|Default|GetCurrent_Inflate))))
    (:then_1
      (Variables|Default|SetTarget_Inflate (Math|Float|Clamp(Float) (+ Inflate_amount (Variables|Default|GetTarget_Inflate)) 0.0 (Variables|Default|GetMax_Inflate))))))

(fn UpdateCurrentInflation
  (params (TimeDelta :type Float%20%28double-precision%29))
  (if (< (Variables|Default|GetCurrent_Inflate) (Variables|Default|GetTarget_Inflate))
    (Variables|Default|SetCurrent_Inflate (Math|Float|Clamp(Float) (+ (Variables|Default|GetCurrent_Inflate) (* (Variables|Default|GetInflationRate) TimeDelta)) 0.0 (Variables|Default|GetMax_Inflate)))
    (Utilities|FlowControl|Sequence
      (:then_0
        (if (== (Variables|Default|GetCurrent_Inflate) (Variables|Default|GetMax_Inflate))
          (Default|CallHitMax)))
      (:then_1
        (if (>= (Variables|Default|GetCurrent_Inflate) (Variables|Default|GetTarget_Inflate))
          (Variables|Default|SetTarget_Inflate 0.0))))
    (elif (> (Variables|Default|GetCurrent_Inflate) (Variables|Default|GetTarget_Inflate))
      (Variables|Default|SetCurrent_Inflate (Math|Float|Clamp(Float) (+ (Variables|Default|GetCurrent_Inflate) (* (Variables|Default|GetDeflate_Rate) TimeDelta -1.0)) 0.0 (Variables|Default|GetMax_Inflate))))))

(fn UpdateMorph
  (Components|SkeletalMesh|SetMorphTarget (Variables|Default|GetInflateMesh) "Inflate" (/ (Variables|Default|GetCurrent_Inflate) (Variables|Default|GetMax_Inflate)) true))

(fn UpdatePhysics
  (Variables|/Script/Engine.PhysicsThrusterComponent|SetThrustStrength (Variables|Default|GetThruster) (Math|Float|Lerp 0.0 (+ (* (Physics|GetMass (Variables|Default|GetInflateMesh)) 5e+02) 1e+03) (/ (Variables|Default|GetCurrent_Inflate) (Variables|Default|GetZero_Weight_Limit))))
  (Components|Activation|SetActive (Variables|Default|GetThruster) true false))