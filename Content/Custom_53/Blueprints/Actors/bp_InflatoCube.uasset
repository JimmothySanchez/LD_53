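; bp_InflatoCube is an inflatable cube actor that bursts into broken planks.
; It forwards received inflate amounts to ACInflateComponent, which is given the cube's skeletal mesh on BeginPlay.
; When the component reports hitting its maximum, the cube ignores all collision, spawns a random number of randomly placed and rotated BP_BrokenPlank actors, pushes each with a fixed impulse, then destroys itself.
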(event Custom|CustomEvent
  (Collision|SetCollisionResponsetoAllChannels (Variables|Default|GetSkel_Inflato_Cube) "ECR_Ignore")
  (for _index (range 0 (Math|Random|RandomIntegerinRange 2 5))
    (bind _returnvalue (Game|SpawnActorfromClass "/Game/Custom_53/Blueprints/Actors/BP_BrokenPlank.BP_BrokenPlank_C" (Math|Transform|MakeTransform (Math|Random|RandomPointinBoundingBox (Transformation|GetActorLocation) "100.000000,100.000000,100.000000") (Math|Random|RandomRotator false)) "Undefined" 0 0))
    (Physics|AddImpulseatLocation (Variables|/Game/Custom_53/Blueprints/Actors/BP_BrokenPlank.BP_BrokenPlank_C|GetBrokenPlank _returnvalue) "1000.000000,1000.000000,1000.000000" (Transformation|GetActorLocation) "None"))
  (Actor|DestroyActor))

(event EventBeginPlay
  (Variables|/Game/Custom_53/Blueprints/Logic/AC_Inflate_Component.AC_Inflate_Component_C|SetInflateMesh (Variables|Default|GetAC_Inflate_Component) (Variables|Default|GetSkel_Inflato_Cube))
  (EventDispatchers|BindEventtoHitMax (Variables|Default|GetAC_Inflate_Component) (delegate Custom|CustomEvent)))

(event Collision|EventActorBeginOverlap
  (params (OtherActor :type Actor%20Object%20Reference)))

(event EventTick
  (params (DeltaSeconds :type Float%20%28single-precision%29)))

(event EventRecieveInflate
  (params (Inflate_Amount :type Float%20%28double-precision%29))
  (Default|AddInflate (Variables|Default|GetAC_Inflate_Component) Inflate_Amount))

(fn ConstructionScript)